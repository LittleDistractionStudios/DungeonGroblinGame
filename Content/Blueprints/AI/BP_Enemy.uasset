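; Enemy Blueprint with health, a hurt state and death, linked to a health bar widget component.
; BeginPlay passes itself to the HealthbarHUD widget and sets starting health.
; TakeDamage subtracts a fixed, clamped amount and flags Hurt, then either clears the flag after a short delay or sets Dead and destroys the actor after a delay.
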(event `Death`
  (`KismetSystemLibrary.Delay` 2.0)
  (`self.K2_DestroyActor`))

(event `ResetHurt`
  (`KismetSystemLibrary.Delay` 0.7)
  (set `self.Hurt` false))

(event `self.ReceiveBeginPlay`
  (bind _ashealthbar_hud (cast `/Game/Blueprints/UI/HealthbarHUD` (`WidgetComponent.GetUserWidgetObject` (`self.HealthBar`))))
  (set `/Game/Blueprints/UI/HealthbarHUD.CharacterRef` self _ashealthbar_hud)
  (set `self.EnemyMaxHealth` 100.0)
  (set `self.EnemyHealth` 100.0))

(fn `TakeDamage`
  (set `self.EnemyHealth` (`KismetMathLibrary.FClamp` (- (`self.EnemyHealth`) 10.0) 0.0 (`self.EnemyMaxHealth`)))
  (set `self.Hurt` true)
  (if (== (`self.EnemyHealth`) 0.0)
    (set `self.Dead` true)
    (`self.Death`)
    (else
      (`self.ResetHurt`))))

(fn `UserConstructionScript`)